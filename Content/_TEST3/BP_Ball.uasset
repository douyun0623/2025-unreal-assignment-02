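; BP_Ball is a ball that a Granny character picks up and throws, exploding on actors that implement BPI_hit.
; PickUp attaches it to the "Ball" mesh socket without collision, while Throw destroys it and spawns a fresh copy with the given velocity.
; BeginPlay launches the projectile movement, then sets blocking collision after a short delay.
; Valid hits spawn an explosion, pass the ball's material through HitMessage and destroy the ball.
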(event `self.ReceiveBeginPlay`
  (bind _projectilemovement (`self.ProjectileMovement`))
  (set `MovementComponent.Velocity` (`self.initial velocity`) _projectilemovement)
  (`ActorComponent.Activate` _projectilemovement false)
  (`KismetSystemLibrary.Delay` 0.2)
  (`PrimitiveComponent.SetCollisionProfileName` (`self.StaticMeshComponent`) "BlockAllDynamic" true))

(event `self.StaticMeshComponent.OnComponentHit`
  (params (HitComponent :type "PrimitiveComponent Object Reference") (OtherActor :type "Actor Object Reference") (OtherComp :type "PrimitiveComponent Object Reference") (NormalImpulse :type "Vector Structure") (Hit :type "HitResult Structure (by ref)"))
  (if (`KismetSystemLibrary.DoesImplementInterface` OtherActor "/Game/_TEST3/BPI/BPI_hit.BPI_hit_C")
    (`GameplayStatics.SpawnEmitterAtLocation` "/Game/StarterContent/Particles/P_Explosion.P_Explosion" (`self.K2_GetActorLocation`) (struct) (1.0 1.0 1.0) true "ManualRelease")
    (message `/Game/_TEST3/BPI/BPI_hit.hit` OtherActor (`PrimitiveComponent.GetMaterial` (`self.StaticMeshComponent`) 0))
    (`self.K2_DestroyActor`)))

(fn `PickUp`
  (params (player :type "Actor Object Reference"))
  (returns (ok :type Boolean))
  (bind _asgranny (cast `/Game/_TEST3/Granny` player))
  (`self.K2_AttachToComponent` (`Character.Mesh` _asgranny) "Ball" "SnapToTarget" "SnapToTarget" "SnapToTarget")
  (`PrimitiveComponent.SetCollisionProfileName` (`self.StaticMeshComponent`) "NoCollision" true)
  (return true))

(fn `Throw`
  (params (location :type "Vector Structure") (velocity :type "Vector Structure"))
  (returns (ok :type Boolean))
  (`self.K2_DetachFromActor` "KeepWorld" "KeepWorld" "KeepWorld")
  (`self.K2_DestroyActor`)
  (`|SpawnActorFromClass` "BP_Ball_C" (`KismetMathLibrary.Conv_VectorToTransform` location) "AlwaysSpawn" "MultiplyWithRoot" null velocity null)
  (return false))

(fn `UserConstructionScript`)