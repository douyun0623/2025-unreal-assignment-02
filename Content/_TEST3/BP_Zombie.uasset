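; BP_Zombie is a zombie character that shuffles slowly forward until hit, and can then be killed.
; BeginPlay loops the walk animation, and Tick adds forward movement input while the Hit flag is false.
; The Hit event swaps in a passed material, stops the animation and sets the flag.
; Death works only once hit, playing the death animation, disabling capsule collision and destroying the actor after a delay.
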(event `self.ReceiveBeginPlay`
  (`SkeletalMeshComponent.PlayAnimation` (`self.Mesh`) "/Game/Characters/Zombie/Animations/Zombie_Walk.Zombie_Walk" true))

(event `self.ReceiveTick`
  (params (DeltaSeconds :type "Float (single-precision)"))
  (if (not (`self.Hit?`))
    (`self.AddMovementInput` (`self.GetActorForwardVector`) 0.05)))

(event `/Game/_TEST3/BPI/BPI_hit.hit`
  (params (Materail :type "MaterialInterface Object Reference"))
  (`PrimitiveComponent.SetMaterial` (`self.Mesh`) 0 Materail)
  (`SkeletalMeshComponent.Stop` (`self.Mesh`))
  (set `self.Hit?` true))

(event `/Game/_TEST3/BPI/BPI_death.death`
  (if (`self.Hit?`)
    (`SkeletalMeshComponent.PlayAnimation` (`self.Mesh`) "/Game/Characters/Zombie/Animations/Zombie_Death.Zombie_Death" false)
    (`PrimitiveComponent.SetCollisionEnabled` (`self.CapsuleComponent`) "NoCollision")
    (`KismetSystemLibrary.Delay` 3.0)
    (`self.K2_DestroyActor`)))

(fn `UserConstructionScript`)